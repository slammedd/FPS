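; BP_Screwdriver is a grabbable tool that removes screws in the world.
; The first grab shows a one-time dialogue line on the first-person character, and a function returns its min and max grab distances.
; Interact runs a debug-drawn sphere trace around the mesh and calls Unscrew on a hit BP_Screw.
; A DoOnce inside the hit loop, reset afterwards, limits each interaction to one screw.
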(event EventBeginPlay)

(event Collision|EventActorBeginOverlap
  (params (OtherActor :type Actor%20Object%20Reference)))

(event EventTick
  (params (DeltaSeconds :type Float%20%28single-precision%29)))

(event EventGrab
  (Utilities|FlowControl|DoOnce false
    (:Completed
      (bind _asbp_first_person_character (Utilities|Casting|CastToBP_FirstPersonCharacter (Game|GetPlayerCharacter 0)))
      (Default|SingleDialogueLine _asbp_first_person_character "Screwdriver...Hm..." 3.0))))

(event EventInteract
  (bind _staticmesh (Variables|Default|GetStaticMesh))
  (bind _returnvalue (Transformation|GetWorldLocation _staticmesh))
  (bind _outhits (Collision|MultiSphereTraceByChannel _returnvalue _returnvalue 25.0 "TraceTypeQuery1" false 0 "ForDuration"))
  (for _array_element _outhits
    (bind _asbp_screw (Utilities|Casting|CastToBP_Screw (.HitActor (Collision|BreakHitResult _array_element))))
    (Utilities|FlowControl|DoOnce false
      (:Completed
        (Default|Unscrew _asbp_screw))))
  (Utilities|FlowControl|DoOnce false) ; enters at Reset
)

(fn ConstructionScript)

(fn ReturnGrabDistances
  (return (Variables|Default|GetMin%20Grab%20Distance) (Variables|Default|GetMax%20Grab%20Distance)))