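; BP_Screw is a removable screw actor, apparently part of a toilet panel puzzle.
; An Unscrew event runs once while CanUnscrew is set, playing a sound and a Remove timeline that rotates and slides the mesh along X.
; When the timeline finishes, the screw starts simulating physics and notifies BP_FirstPersonGameMode through ToiletPanelScrewRemoved.
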(event Custom|Unscrew
  (bind _staticmesh (Variables|Default|GetStaticMesh))
  (if (Variables|Default|GetCan%20Unscrew)
    (Variables|Default|SetCan%20Unscrew false)
    (Audio|PlaySoundatLocation "/Game/Audio/SC_Unscrew.SC_Unscrew" (Transformation|GetActorLocation) "0, 0, 0" 1.0 1.0 0.0 0 0 0 0)
    (bind (_direction _x_rotation _x_location) (Timeline|Remove Play)
      (:Update
        (Transformation|SetRelativeRotation _staticmesh (Math|Rotator|MakeRotator _x_rotation 0.0 0.0) false false)
        (Transformation|SetRelativeLocation _staticmesh (Math|Vector|MakeVector _x_location 0.0 0.0) false false))
      (:Finished
        (Physics|SetSimulatePhysics _staticmesh true)
        (bind _asbp_first_person_game_mode (Utilities|Casting|CastToBP_FirstPersonGameMode (Game|GetGameMode)))
        (Default|ToiletPanelScrewRemoved _asbp_first_person_game_mode)))))

(fn ConstructionScript)