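; Interactable light switch that toggles a set of three spotlights, tube meshes and hum sounds together.
; Interact flips between SwitchOn and SwitchOff based on SwitchedOn, and BeginPlay applies the OnByDefault state.
; Each direction has its own timeline that pitches the Pivot.
; When the timeline finishes, it updates SwitchedOn, plays the switch click, sets spotlight visibility, swaps tube materials and fades the hums.
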(event Custom|Switch%20On
  (bind _y_rotation (Timeline|Turn%20On PlayFromStart)
    (:Update
      (Transformation|SetRelativeRotation (Variables|Default|GetPivot) (Math|Rotator|MakeRotator 0.0 _y_rotation 0.0) false false))
    (:Finished
      (Variables|Default|SetSwitched%20On true)
      (Audio|PlaySoundatLocation "/Game/Audio/SC_Light_Switch.SC_Light_Switch" (Transformation|GetActorLocation) "0, 0, 0" 1.0 1.0 0.0 0 0 0 0)
      (Rendering|SetVisibility (Variables|Default|GetSpotLight) true false)
      (Rendering|Material|SetMaterial (Variables|Default|GetLight%20Tubes) 0 "/Game/Meshes/Ceiling_Light/MAT_Tube_Inst.MAT_Tube_Inst")
      (Audio|Components|Audio|FadeIn (Variables|Default|GetLight_Hum) 0.1 1.0 0.0 "Linear" :!class /Script/Engine.AudioComponent))))

(event Custom|Switch%20Off
  (bind _y_rotation (Timeline|Timeline ReverseFromEnd)
    (:Update
      (Transformation|SetRelativeRotation (Variables|Default|GetPivot) (Math|Rotator|MakeRotator 0.0 _y_rotation 0.0) false false))
    (:Finished
      (Variables|Default|SetSwitched%20On false)
      (Audio|PlaySoundatLocation "/Game/Audio/SC_Light_Switch.SC_Light_Switch" (Transformation|GetActorLocation) "0, 0, 0" 1.0 1.0 0.0 0 0 0 0)
      (Rendering|SetVisibility (Variables|Default|GetSpotLight) false false)
      (Rendering|Material|SetMaterial (Variables|Default|GetLight%20Tubes) 0 "/Game/Meshes/Ceiling_Light/MAT_Tube_Off.MAT_Tube_Off")
      (Audio|Components|Audio|FadeOut (Variables|Default|GetLight_Hum) 0.1 0.0 "Linear" :!class /Script/Engine.AudioComponent))))

(event EventBeginPlay
  (Audio|Components|Audio|Stop (Variables|Default|GetLight_Hum))
  (if (Variables|Default|GetOn%20by%20Default)
    (CallFunction|Switchon)
    (else
      (CallFunction|SwitchOff))))

(event EventInteract
  (if (Variables|Default|GetSwitched%20On)
    (CallFunction|SwitchOff)
    (else
      (CallFunction|Switchon))))

(fn ConstructionScript)