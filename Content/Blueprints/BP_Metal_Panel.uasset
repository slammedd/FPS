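; BP_Metal_Panel is a screwed-down metal panel that the player can grab once it has been unscrewed.
; Unscrewed enables grabbing, turns on mesh physics and has BP_FirstPersonCharacter show a line about a way out.
; Grab plays a "screwed tight" line while locked, or a one-time remark on the weight once loose.
; ReturnGrabDistances supplies the minimum grab distance, with the maximum left at zero.
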(event Custom|Unscrewed
  (Variables|Default|SetCan%20Grab true)
  (Physics|SetSimulatePhysics (Variables|Default|GetStaticMesh) true)
  (bind _asbp_first_person_character (Utilities|Casting|CastToBP_FirstPersonCharacter (Game|GetPlayerCharacter 0)))
  (Default|SingleDialogueLine _asbp_first_person_character "A way out..." 2.5))

(event EventGrab
  (if (Variables|Default|GetCan%20Grab)
    (Utilities|FlowControl|DoOnce false
      (:Completed
        (bind _asbp_first_person_character (Utilities|Casting|CastToBP_FirstPersonCharacter (Game|GetPlayerCharacter 0)))
        (Default|SingleDialogueLine _asbp_first_person_character "Jesus that's heavy." 1.5)))
    (else
      (bind _asbp_first_person_character_2 (Utilities|Casting|CastToBP_FirstPersonCharacter (Game|GetPlayerCharacter 0)))
      (Default|SingleDialogueLine _asbp_first_person_character_2 "Seems screwed tight." 1.5))))

(fn ConstructionScript)

(fn ReturnGrabDistances
  (return (Variables|Default|GetMin%20Grab%20Distance) 0.0))