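; BP_Backpack is a grabbable, interactable backpack prop that yields a screwdriver.
; The first Grab shows a player dialogue line hinting that it isn't empty.
; Interact plays an opening sound, swaps to the open mesh, shows a reaction line and spawns BP_Screwdriver at ScrewdriverSpawnPoint, with no once-only guard in this graph.
; ReturnGrabDistances supplies the minimum and maximum grab distances.
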(event EventBeginPlay)

(event Collision|EventActorBeginOverlap
  (params (OtherActor :type Actor%20Object%20Reference)))

(event EventTick
  (params (DeltaSeconds :type Float%20%28single-precision%29)))

(event EventInteract
  (Audio|PlaySoundatLocation "/Game/Audio/SC_Backpack_Open.SC_Backpack_Open" (Transformation|GetActorLocation) "0, 0, 0" 1.0 1.0 0.0 0 0 0 0)
  (Components|StaticMesh|SetStaticMesh (Variables|Default|GetStaticMesh) "/Game/Meshes/Backpack/Backpack_Open.Backpack_Open")
  (bind _asbp_first_person_character (Utilities|Casting|CastToBP_FirstPersonCharacter (Game|GetPlayerCharacter 0)))
  (Default|SingleDialogueLine _asbp_first_person_character "Woah!" 1.5)
  (Game|SpawnActorfromClass "/Game/Blueprints/BP_Screwdriver.BP_Screwdriver_C" (Transformation|GetWorldTransform (Variables|Default|GetScrewdriver%20Spawn%20Point)) "Undefined" "MultiplyWithRoot" 0 0))

(event EventGrab
  (Utilities|FlowControl|DoOnce false
    (:Completed
      (bind _asbp_first_person_character (Utilities|Casting|CastToBP_FirstPersonCharacter (Game|GetPlayerCharacter 0)))
      (Default|SingleDialogueLine _asbp_first_person_character "Backpack... Doesn't feel empty." 3.0))))

(fn ConstructionScript)

(fn ReturnGrabDistances
  (return (Variables|Default|GetMin%20Grab%20Distance) (Variables|Default|GetMax%20Grab%20Distance)))